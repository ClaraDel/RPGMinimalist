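; Interactive spotlight actor that the player switches on and off with the F key while inside its box trigger.
; Box begin and end overlap enable or disable input for player controller 0 and flip the FToggle component's visibility, with no check on which actor overlaps.
; The construction script applies the Color and Visibility variables to the spotlight, setting its color and initial state per instance.
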(event OnComponentBeginOverlap(Box)
  (params (OverlappedComponent :type Primitive%20Component%20Object%20Reference) (OtherActor :type Actor%20Object%20Reference) (OtherComp :type Primitive%20Component%20Object%20Reference) (OtherBodyIndex :type Integer) (bFromSweep :type Boolean) (SweepResult :type Hit%20Result%20Structure%20%28by%20ref%29))
  ;[0.8844 0.3565 0.6203] Coucou Quentin
  (Input|EnableInput (Game|GetPlayerController 0))
  (Rendering|ToggleVisibility (Variables|Default|GetFToggle) false))

(event OnComponentEndOverlap(Box)
  (params (OverlappedComponent :type Primitive%20Component%20Object%20Reference) (OtherActor :type Actor%20Object%20Reference) (OtherComp :type Primitive%20Component%20Object%20Reference) (OtherBodyIndex :type Integer))
  ;[0.8844 0.3565 0.6203] Coucou Quentin
  (Input|DisableInput (Game|GetPlayerController 0))
  (Rendering|ToggleVisibility (Variables|Default|GetFToggle) false))

(event EventBeginPlay)

(event Collision|EventActorBeginOverlap
  (params (OtherActor :type Actor%20Object%20Reference)))

(event EventTick
  (params (DeltaSeconds :type Float%20%28single-precision%29)))

(event Input|KeyboardEvents|F
  (params (Key :type Key%20Structure :default "None"))
  ;[0.8844 0.3565 0.6203] Coucou Quentin
  (:Pressed
    (Rendering|ToggleVisibility (Variables|Default|GetSpotLight) false)))

(fn ConstructionScript
  (bind _spotlight (Variables|Default|GetSpotLight))
  (Rendering|Components|Light|SetLightColor _spotlight (Variables|Default|GetColor) true)
  (Rendering|SetVisibility _spotlight (Variables|Default|GetVisibility) false))